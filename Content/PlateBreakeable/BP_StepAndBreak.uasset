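; BP_StepAndBreak is a configurable breakable prop that gives the player away with noise when stepped on.
; Its construction script applies the chosen mesh and trigger box extent.
; Box overlap by BP_PDPlayerCharacter emits noise at the player's location, plays a break sound, activates particles, then destroys the actor after a configurable delay.
; An unconnected SetAsset node for the particles never runs.
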(event OnComponentBeginOverlap(Box)
  (params (OverlappedComponent :type Primitive%20Component%20Object%20Reference) (OtherActor :type Actor%20Object%20Reference) (OtherComp :type Primitive%20Component%20Object%20Reference) (OtherBodyIndex :type Integer) (bFromSweep :type Boolean) (SweepResult :type Hit%20Result%20Structure%20%28by%20ref%29))
  (bind _asbp_pdplayer_character (Utilities|Casting|CastToBP_PDPlayerCharacter OtherActor))
  (bind _output_get (Variables|Default|SetBP%20PDPlayer%20Character _asbp_pdplayer_character))
  (Class|Actor|MakeNoise 1.0 _output_get (Transformation|GetActorLocation (Variables|Default|GetBP%20PDPlayer%20Character)) 0.0 "None")
  (Audio|PlaySoundatLocation (Variables|Default|GetSoundToPlayOnBreak) (Transformation|GetActorLocation) "0, 0, 0" 1.0 1.0 0.0 0 0 0 0)
  (Components|Activation|Activate (Variables|Default|GetParticlesToSpawnOnBreak) true)
  (Utilities|FlowControl|Delay (Variables|Default|GetTimeForTheObjectToDissapear))
  (Actor|DestroyActor))

(event EventBeginPlay)

(event Collision|EventActorBeginOverlap
  (params (OtherActor :type Actor%20Object%20Reference)))

(event EventTick
  (params (DeltaSeconds :type Float%20%28single-precision%29)))

(fn ConstructionScript
  (Components|Box|SetBoxExtent (Variables|Default|GetBox) (Variables|Default|GetBoxExtent) true)
  (Components|StaticMesh|SetStaticMesh (Variables|Default|GetStaticMesh) (Variables|Default|GetMesh)))