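; Base enemy Character Blueprint that provides attack, patrol route and movement speed functions.
; Attack plays the Zlorp attack montage on the mesh and fires the OnAttackEnd dispatcher whether the montage completes or is interrupted.
; GetPatrolRoute exposes the assigned route, and SetMovementSpeed maps an idle-to-sprint speed state to the CharacterMovement max walk speed and returns it.
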(event Custom|Attack
  (Animation|Montage|PlayMontage (Variables|Character|GetMesh) "/Game/Enemy/Animations/Attack/AM_ZlorpAttack1.AM_ZlorpAttack1"
    (:OnCompleted
      _)
    (:OnInterrupted
      _))
  (Default|CallOnAttackEnd))

(fn ConstructionScript)

(fn GetPatrolRoute
  (return (Variables|AI|GetPatrolRoute)))

(fn SetMovementSpeed
  (params (Speed :type E_MovementSpeed%20Enum :default "NewEnumerator0"))
  (bind _output_get (Variables|/Script/Engine.CharacterMovementComponent|SetMaxWalkSpeed (Variables|Character|GetCharacterMovement) (Utilities|Select :Index Speed :NewEnumerator0 0.0 :NewEnumerator1 2.5e+02 :NewEnumerator2 6e+02 :NewEnumerator3 8.5e+02)))
  (return _output_get))