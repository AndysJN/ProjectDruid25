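; Enemy AI controller that runs BT_EnemyBase and switches its blackboard state between Passive, Investigating and Combat using AI perception.
; Seeing the player with an active torch starts combat, while a heard noise triggers investigation of its location, both ignored during combat.
; A looping timer compares seen actors against perception's known sight actors, returning to Passive when the player is forgotten.
; A damage handler can also start combat, but nothing here calls it.
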(event OnPerceptionUpdated(AIPerception)
  (params (UpdatedActors :type Array%20of%20Actor%20Object%20References))
  (for _array_element UpdatedActors
    (Utilities|FlowControl|Sequence
      (:then_0
        (bind _sensedactor (CallFunction|CanSenseActor _array_element "NewEnumerator1"))
        (if _sensedactor
          (CallFunction|HandleSensedSight _array_element)))
      (:then_1
        (bind (_sensedactor_2 _stimilusobject) (CallFunction|CanSenseActor _array_element "NewEnumerator2"))
        (if _sensedactor_2
          (CallFunction|HandleSensedSound (.StimulusLocation (Utilities|Struct|BreakAIStimulus _stimilusobject))))))))

(event Custom|CheckIfPlayerForgotten
  (if (!= (Utilities|Array|Length (Class|AIPerceptionComponent|GetKnownPerceivedActors (Variables|Default|GetAIPerception) "/Script/AIModule.AISense_Sight")) (Utilities|Array|Length (Variables|Default|GetSeenActors)))
    (for _array_element (Variables|Default|GetSeenActors)
      (if (== (Utilities|Array|FindItem (Class|AIPerceptionComponent|GetKnownPerceivedActors (Variables|Default|GetAIPerception) "/Script/AIModule.AISense_Sight") _array_element) -1)
        (CallFunction|HandleForgotActor _array_element)))))

(event EventUnPossess
  (params (UnpossessedPawn :type Pawn%20Object%20Reference))
  (Utilities|Time|ClearandInvalidateTimerbyHandle (Variables|Default|GetCheckForgottenPlayerTimer)))

(event EventPossess
  (params (PossessedPawn :type Pawn%20Object%20Reference))
  (AI|RunBehaviorTree "/Game/Enemy/AI/BT_EnemyBase.BT_EnemyBase")
  (CallFunction|SetStateasPassive)
  (bind _returnvalue (Utilities|Time|SetTimerbyEvent (EventDispatchers|CreateEvent :!event Custom|CheckIfPlayerForgotten) 0.5 true))
  (Variables|Default|SetCheckForgottenPlayerTimer _returnvalue))

(fn ConstructionScript)

(fn SetStateasPassive
  (AI|Components|Blackboard|SetValueasEnum (Variables|Default|GetBlackboard) (Variables|Default|GetStateKeyName) (Utilities|Enum|LiteralenumE_AIState "NewEnumerator0")))

(fn SetStateasCombat
  (params (AttackTarget :type Actor%20Object%20Reference))
  (AI|Components|Blackboard|SetValueasObject (Variables|Default|GetBlackboard) (Variables|Default|GetAttackTargetKeyName) AttackTarget)
  (AI|Components|Blackboard|SetValueasEnum (Variables|Default|GetBlackboard) (Variables|Default|GetStateKeyName) (Utilities|Enum|LiteralenumE_AIState "NewEnumerator1")))

(fn CanSenseActor
  (params (ActorToSense :type Actor%20Object%20Reference) (TypeToSense :type E_AISenseType%20Enum :default "NewEnumerator0"))
  (bind _info (Class|AIPerceptionComponent|GetActorsPerception (Variables|Default|GetAIPerception) ActorToSense))
  (for _array_element (.LastSensedStimuli (Utilities|Struct|BreakActorPerceptionBlueprintInfo _info))
    (bind _returnvalue (Class|AIPerceptionSystem|GetSenseClassforStimulus _array_element))
    (if (== _returnvalue (Utilities|Select :Index TypeToSense :NewEnumerator0 0 :NewEnumerator1 "/Script/AIModule.AISense_Sight" :NewEnumerator2 "/Script/AIModule.AISense_Hearing" :NewEnumerator3 "/Script/AIModule.AISense_Damage"))
      (return (.bSuccessfullySensed (Utilities|Struct|BreakAIStimulus _array_element)) _array_element))))

(fn HandleSensedSight
  (params (SensedActor :type Actor%20Object%20Reference))
  (Utilities|Array|AddUnique (Variables|Default|GetSeenActors) SensedActor)
  (bind _asbp_pdplayer_character (Utilities|Casting|CastToBP_PDPlayerCharacter SensedActor))
  (Variables|Default|SetBP%20PDPlayer%20Character _asbp_pdplayer_character)
  (bind _statename (CallFunction|GetCurrentState))
  (switch Utilities|FlowControl|Switch|SwitchonE_AIState _statename
    (:NewEnumerator0
      _)
    (:NewEnumerator2
      _))
  (if (Variables|/Script/ProjectDruid.PDPlayerCharacter|GetbTorchActive (Variables|Default|GetBP%20PDPlayer%20Character))
    (CallFunction|SetStateasCombat (Variables|Default|GetBP%20PDPlayer%20Character))))

(fn GetCurrentState
  (return (Utilities|Enum|ByteToEnumE_AIState (Class|BlackboardComponent|GetValueasEnum (Variables|Default|GetBlackboard) (Variables|Default|GetStateKeyName)))))

(fn HandleSensedSound
  (params (SoundLocation :type Vector))
  (bind _statename (CallFunction|GetCurrentState))
  (switch Utilities|FlowControl|Switch|SwitchonE_AIState _statename
    (:NewEnumerator0
      _)
    (:NewEnumerator2
      _))
  (CallFunction|SetStateasInvestigating SoundLocation))

(fn SetStateasInvestigating
  (params (Location :type Vector))
  (AI|Components|Blackboard|SetValueasEnum (Variables|Default|GetBlackboard) (Variables|Default|GetStateKeyName) (Utilities|Enum|LiteralenumE_AIState "NewEnumerator2"))
  (AI|Components|Blackboard|SetValueasVector (Variables|Default|GetBlackboard) (Variables|Default|GetLocationKeyName) Location))

(fn HandleSensedDamage
  (params (DamageCauser :type Actor%20Object%20Reference))
  (bind _statename (CallFunction|GetCurrentState))
  (switch Utilities|FlowControl|Switch|SwitchonE_AIState _statename
    (:NewEnumerator0
      _)
    (:NewEnumerator2
      _))
  (CallFunction|SetStateasCombat DamageCauser))

(fn HandleForgotActor
  (params (Actor :type Actor%20Object%20Reference))
  (Utilities|Array|RemoveItem (Variables|Default|GetSeenActors) 0)
  (if (== Actor (Variables|Default|GetBP%20PDPlayer%20Character))
    (CallFunction|SetStateasPassive)))