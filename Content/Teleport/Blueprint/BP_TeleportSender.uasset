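; Teleport pad actor that moves the player character to a Target actor's location, slightly raised, when they overlap its box.
; Input is disabled while dynamic instances of a teleport effect material replace the mesh's first two material slots.
; Two chained timelines animate the material's Edge parameter out, then in, with the move between them.
; Afterwards it restores the materials cached at BeginPlay and re-enables input.
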(event OnComponentBeginOverlap(Box)
  (params (OverlappedComponent :type Primitive%20Component%20Object%20Reference) (OtherActor :type Actor%20Object%20Reference) (OtherComp :type Primitive%20Component%20Object%20Reference) (OtherBodyIndex :type Integer) (bFromSweep :type Boolean) (SweepResult :type Hit%20Result%20Structure%20%28by%20ref%29))
  (bind _returnvalue (Game|GetPlayerController 0))
  (bind _returnvalue_2 (Game|GetPlayerController 0))
  (bind _target (Variables|Default|GetTarget))
  (bind _returnvalue_3 (Transformation|GetActorLocation _target))
  (Utilities|Casting|CastToBP_PDPlayerCharacter OtherActor)
  (Input|DisableInput _returnvalue _returnvalue)
  (bind _output_get (Variables|Default|SetPlayerMesh (Variables|/Script/Engine.Character|GetMesh (Variables|Default|GetPlayerCharacter))))
  (bind _returnvalue_4 (Rendering|Material|CreateDynamicMaterialInstance _output_get 0 "/Game/Teleport/Materials/MI_TeleportEffect.MI_TeleportEffect" "None" :!class /Script/Engine.PrimitiveComponent))
  (Variables|Default|SetDMI_0 _returnvalue_4)
  (bind _returnvalue_5 (Rendering|Material|CreateDynamicMaterialInstance (Variables|Default|GetPlayerMesh) 1 "/Game/Teleport/Materials/MI_TeleportEffect.MI_TeleportEffect" "None" :!class /Script/Engine.PrimitiveComponent))
  (Variables|Default|SetDMI_1 _returnvalue_5)
  (bind _edge (Timeline|TeleportOut PlayFromStart)
    (:Update
      (Rendering|Material|SetScalarParameterValue (Variables|Default|GetDMI_0) "Edge" _edge :!class /Script/Engine.MaterialInstanceDynamic))
    (:Finished
      (Transformation|SetActorLocation (Variables|Default|GetPlayerCharacter) (Math|Vector|MakeVector (.x _returnvalue_3) (.y _returnvalue_3) (+ (.z _returnvalue_3) 1e+02)) false false)
      (bind _edge_2 (Timeline|TeleportIn PlayFromStart)
        (:Update
          (Rendering|Material|SetScalarParameterValue (Variables|Default|GetDMI_0) "Edge" _edge_2 :!class /Script/Engine.MaterialInstanceDynamic))
        (:Finished
          (for (_array_element _array_index) (Variables|Default|GetPlayerMaterials)
            (Rendering|Material|SetMaterial (Variables|Default|GetPlayerMesh) _array_index _array_element))
          (Input|EnableInput _returnvalue_2 _returnvalue_2))))))

(event EventBeginPlay
  ;[0.15 0.15 0.15 0.5] Get Ref to Player Character
  (bind _asbp_pdplayer_character (Utilities|Casting|CastToBP_PDPlayerCharacter (Game|GetPlayerCharacter 0)))
  (bind _output_get (Variables|Default|SetPlayerCharacter _asbp_pdplayer_character))
  (Variables|Default|SetPlayerMaterials (Rendering|Material|GetMaterials (Variables|/Script/Engine.Character|GetMesh _output_get))))

(fn ConstructionScript)